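; BP_SubtitulosWini is a Blueprint that displays a subtitle widget on screen.
; On BeginPlay it creates a Subtitulos widget, stores it and adds it to the viewport.
; Tick polls the IsActivated flag every frame to show or hide the widget; nothing in this Blueprint sets the flag.
; The node that copies the Subtitul variable into the widget's text block is unconnected, so that text is never applied.
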(event EventBeginPlay
  (bind _returnvalue (UserInterface|CreateWidget "/Game/art/WINI/Subtitulos/Subtitulos.Subtitulos_C"))
  (bind _output_get (Variables|Default|SetSubtitulos _returnvalue))
  (UserInterface|Viewport|AddtoViewport _output_get 0))

(event Collision|EventActorBeginOverlap
  (params (OtherActor :type Actor%20Object%20Reference)))

(event EventTick
  (params (DeltaSeconds :type Float%20%28single-precision%29))
  (if (Variables|Default|GetIsActivated)
    (Variables|/Script/UMG.Widget|SetVisibility (Variables|Default|GetSubtitulos) "Visible")
    (else
      (Variables|/Script/UMG.Widget|SetVisibility (Variables|Default|GetSubtitulos) "Hidden"))))

(fn ConstructionScript)