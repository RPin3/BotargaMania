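; BP_Camera is a camera actor that repositions itself from the locations of the actors in its Players list.
; Each Tick it runs GetAllActorsOfClass, then loops over Players, adding each location to a running sum that is never reset in the graph.
; Inside the loop it halves that sum, a fixed two-player divisor, and sets its location through VInterpTo with that value as Current.
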(event EventBeginPlay)

(event Collision|EventActorBeginOverlap
  (params (OtherActor :type Actor%20Object%20Reference)))

(event EventTick
  (params (DeltaSeconds :type Float%20%28single-precision%29))
  (Actor|GetAllActorsOfClass 0)
  (for _array_element (Variables|Default|GetPlayers)
    (bind _output_get (Variables|Default|SetAddPonits (+ (Transformation|GetActorLocation _array_element) (Variables|Default|GetAddPonits))))
    (bind _output_get_2 (Variables|Default|SetMedio (/ _output_get 2.0)))
    (Transformation|SetActorLocation (Math|Interpolation|VInterpTo _output_get_2 "0, 0, 0" 0.0 0.0) false false)))

(fn ConstructionScript)