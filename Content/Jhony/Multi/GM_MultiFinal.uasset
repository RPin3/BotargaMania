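; GM_MultiFinal is a game mode that sets up Player 1 and Player 2 for local multiplayer.
; Each SelectPlayer event sets the default pawn class from DefaultPawnClassN, restarts its indexed player controller, then calls CreatePlayer for that controller ID.
; RestartPlayer runs before CreatePlayer in both events.
; If the controller is valid afterward, it is stored as P1 or P2 and a debug label prints.
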(event Custom|SelectPlayer2
  (bind _returnvalue (Game|GetPlayerController 1))
  (Variables|Default|SetDefaultPawnClass (Variables|Default|GetDefault%20Pawn%20ClassN))
  (Class|GameModeBase|RestartPlayer (Game|GetGameMode) _returnvalue)
  (Class|GameplayStatics|CreatePlayer 1)
  (if (Utilities|IsValid _returnvalue)
    (Variables|Default|SetP2 _returnvalue)
    (Development|PrintString "Player 2" true true "(R=0.000000,G=0.065985,B=1.000000,A=1.000000)" 5.0)))

(event Custom|SelectPlayer1
  (bind _returnvalue (Game|GetPlayerController 0))
  (Variables|Default|SetDefaultPawnClass (Variables|Default|GetDefault%20Pawn%20ClassN))
  (Class|GameModeBase|RestartPlayer (Game|GetGameMode) _returnvalue)
  (Class|GameplayStatics|CreatePlayer 0)
  (if (Utilities|IsValid _returnvalue)
    (Variables|Default|SetP1 _returnvalue)
    (Development|PrintString "Player 1" true true "(R=0.000000,G=0.065985,B=1.000000,A=1.000000)" 5.0)))

(fn ConstructionScript)