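; Player controller Blueprint that sets up player one input and handles a join-game action for local multiplayer.
; Shortly after BeginPlay it adds the IMC_Player1 mapping context through the Enhanced Input local player subsystem.
; The join action creates a second local player with its own controller if this controller has a pawn; otherwise it asks the GameMode to restart this player and prints a controller-loss message.
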(event Input|EnhancedActionEvents|EnhancedInputActionIA_JoinGame
  (params (ActionValue :type Boolean) (ElapsedSeconds :type Float%20%28double-precision%29) (TriggeredSeconds :type Float%20%28double-precision%29) (InputAction :type Input%20Action%20Object%20Reference :default "/Game/ThirdPerson/Input/Actions/IA_JoinGame.IA_JoinGame"))
  (:Started
    (Utilities|IsValid (Pawn|GetControlledPawn)
      (:Is%20Valid
        (Class|GameplayStatics|CreatePlayer 1))
      (:Is%20Not%20Valid
        (Class|GameModeBase|RestartPlayer (Game|GetGameMode) self)
        (Development|PrintString "Controller loss")))))

(event EventBeginPlay
  (bind _self self)
  (bind _returnvalue (PlayerController|LocalPlayerSubsystems|GetEnhancedInputLocalPlayerSubsystem _self))
  (Utilities|FlowControl|Delay 0.5)
  (Utilities|IsValid _returnvalue
    (:Is%20Valid
      (Input|AddMappingContext _returnvalue "/Game/Charater2D/Input/IMC_Player1.IMC_Player1" 0 "(bIgnoreAllPressedKeysUntilRelease=True,bForceImmediately=False,bNotifyUserSettings=False)"))))

(fn ConstructionScript)