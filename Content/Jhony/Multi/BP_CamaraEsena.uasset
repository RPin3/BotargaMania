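; BP_CamaraEsena is a scene camera that follows one or two player characters.
; A Delay in Tick throttles updates to roughly every 0.3 seconds, moving the camera component in unswept steps without interpolation.
; With a valid second player it sits above the midpoint of both characters; otherwise it follows the first at a raised, sideways offset.
; Only location is set, never rotation or zoom.
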(event EventBeginPlay)

(event Collision|EventActorBeginOverlap
  (params (OtherActor :type Actor%20Object%20Reference)))

(event EventTick
  (params (DeltaSeconds :type Float%20%28single-precision%29))
  (bind _returnvalue (Game|GetPlayerCharacter 1))
  (bind _cameracomponent (Variables|CameraActor|GetCameraComponent))
  (Utilities|FlowControl|Delay 0.3)
  (if (Utilities|IsValid _returnvalue)
    (Transformation|SetWorldLocation _cameracomponent (+ "0.000000,0.000000,500.000000" (/ (+ (Transformation|GetWorldLocation (Variables|/Script/Engine.Actor|GetRootComponent _returnvalue)) (Transformation|GetWorldLocation (Variables|/Script/Engine.Actor|GetRootComponent (Game|GetPlayerCharacter 0)))) 2)) false false)
    (else
      (Transformation|SetWorldLocation _cameracomponent (+ (Transformation|GetWorldLocation (Variables|/Script/Engine.Actor|GetRootComponent (Game|GetPlayerCharacter 0))) "0.000000,500.000000,800.000000") false false))))

(fn ConstructionScript)