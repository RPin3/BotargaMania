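; BP_AutoBoom is a Chaos actor that automatically sets off a field on its geometry component after a fixed two-minute delay from BeginPlay.
; It spawns a short-lived MF field actor from the component's relative location, sets its activation type and fires CETrigger.
; The actor then waits for the fragment lifetime and destroys itself.
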(event Collision|EventActorBeginOverlap
  (params (OtherActor :type Actor%20Object%20Reference)))

(event EventTick
  (params (DeltaSeconds :type Float%20%28single-precision%29)))

(event EventBeginPlay
  (bind _geometrycomponent (Variables|Default|GetGeometryComponent))
  (bind _relativelocation (Variables|/Script/Engine.SceneComponent|GetRelativeLocation _geometrycomponent))
  (bind _returnvalue (Math|Conversions|ToTransform(Vector) _relativelocation))
  (Utilities|FlowControl|Delay 1.2e+02)
  (bind _returnvalue_2 (Game|SpawnActorfromClass "/Game/Jhony/Chaos/GC/MF_Base.MF_Base_C" (Math|Transform|MakeTransform (.location _returnvalue) (.rotation _returnvalue) (.scale _returnvalue)) "Undefined" "MultiplyWithRoot" 0 0))
  (bind _output_get (Variables|Default|SetMF _returnvalue_2))
  (Variables|/Engine/EditorResources/FieldNodes/FS_MasterField.FS_MasterField_C|SetActivationType _output_get "NewEnumerator4")
  (Actor|SetLifeSpan (Variables|Default|GetMF) 0.15)
  (Default|CETrigger (Variables|Default|GetMF))
  (Utilities|FlowControl|Delay (Variables|Default|GetFragmentLifeTiem))
  (Actor|DestroyActor))

(fn ConstructionScript)