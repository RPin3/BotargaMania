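; BP_Change is an actor that, when hit, triggers a Chaos field effect and then switches to another level.
; A hit on its GeometryComponent spawns a small, short-lived MF_Base field at the impact point, sets its activation type and fires CETrigger.
; It prints a loading message, waits for LifeTime, then opens the level named by LevelName.
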(event OnComponentHit(GeometryComponent)
  (params (HitComponent :type Primitive%20Component%20Object%20Reference) (OtherActor :type Actor%20Object%20Reference) (OtherComp :type Primitive%20Component%20Object%20Reference) (NormalImpulse :type Vector :default "0, 0, 0") (Hit :type Hit%20Result%20Structure%20%28by%20ref%29))
  (bind _impactpoint (Collision|BreakHitResult Hit))
  (bind _returnvalue (Math|Conversions|ToTransform(Vector) _impactpoint))
  (bind _returnvalue_2 (Game|SpawnActorfromClass "/Game/Jhony/Chaos/GC/MF_Base.MF_Base_C" (Math|Transform|MakeTransform (.location _returnvalue) (.rotation _returnvalue) "0.100000,0.300000,0.300000") "Undefined" "MultiplyWithRoot" 0 0))
  (bind _output_get (Variables|Default|SetMF _returnvalue_2))
  (Variables|/Engine/EditorResources/FieldNodes/FS_MasterField.FS_MasterField_C|SetActivationType _output_get "NewEnumerator4")
  (Actor|SetLifeSpan (Variables|Default|GetMF) 0.1)
  (Default|CETrigger (Variables|Default|GetMF))
  (Development|PrintString "CARGANDO ESENA" true true "(R=0.000000,G=0.134117,B=1.000000,A=1.000000)" 0.1)
  (Utilities|FlowControl|Delay (Variables|Default|GetLifeTime))
  (Game|OpenLevel(byName) (Variables|Default|GetLevel%20Name)))

(event EventBeginPlay)

(event Collision|EventActorBeginOverlap
  (params (OtherActor :type Actor%20Object%20Reference)))

(event EventTick
  (params (DeltaSeconds :type Float%20%28single-precision%29)))

(fn ConstructionScript)