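; Actor component that tracks an owner's health, starting at MaxHealth and broadcasting OnHealthChanged on initialization and each change.
; DamageHealth branches on stored movement Direction: at -1 it sets Health to a tenth of Damage minus Health, otherwise it subtracts full Damage.
; It then prints the value and flags IsDead only when Health equals exactly zero.
; ChangeLife subtracts and broadcasts without that death check.
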(event Custom|Dead
  (if (== (Variables|Default|GetHealth) 0.0)
    (Variables|Default|SetIsDead true)))

(event Custom|ChangeLife
  (params (Damage :type Float%20%28double-precision%29))
  (bind _output_get (Variables|Default|SetHealth (- (Variables|Default|GetHealth) Damage)))
  (Default|CallOnHealthChanged _output_get))

(event EventBeginPlay
  (Variables|Default|SetHealth (Variables|Default|GetMaxHealth))
  (Default|CallOnHealthChanged (Variables|Default|GetHealth)))

(event EventStopMovement
  (params (Movement :type Float%20%28double-precision%29))
  (Variables|Default|SetDirection Movement))

(event EventDamageHealth
  (params (Damage :type Float%20%28double-precision%29))
  (if (== (Variables|Default|GetDirection) -1.0)
    (bind _output_get (Variables|Default|SetHealth (- (* Damage 0.1) (Variables|Default|GetHealth))))
    (Development|PrintString (Utilities|String|ToString(Float) _output_get))
    (Default|CallOnHealthChanged (Variables|Default|GetHealth))
    (else
      (bind _output_get_2 (Variables|Default|SetHealth (- (Variables|Default|GetHealth) Damage)))
      (Development|PrintString (Utilities|String|ToString(Float) _output_get_2))
      (Default|CallOnHealthChanged (Variables|Default|GetHealth))))
  (CallFunction|Dead))

(event EventDirectionMovement
  (params (Direction :type Float%20%28double-precision%29))
  (Variables|Default|SetDirection Direction))