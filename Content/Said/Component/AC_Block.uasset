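; AC_Block is an actor component that handles blocking, passing damage-block values to the owner's BPI_Health component.
; A DirectionMovement input of -1 first sets a Debug flag as the blocking state, then repeated calls send a reduced block value.
; StopMovement clears the flag, looks up the health component by interface and restores the full value.
; The directional branch reuses that lookup result without performing its own.
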(event EventStopMovement
  (params (Movement :type Float%20%28double-precision%29))
  (Development|PrintString "Paro de bloquear")
  (Variables|Default|SetDebug false)
  (bind _component (CallFunction|FindComponentbyInterface (Components|GetOwner) "/Game/Said/Interface/BPI_Health.BPI_Health_C"))
  (Class|BPIHealth|BlockDamage(Message) _component 1.0))

(event EventDirectionMovement
  (params (Direction :type Float%20%28double-precision%29))
  (if (== Direction -1.0)
    (if (Variables|Default|GetDebug)
      (Class|BPIHealth|BlockDamage(Message) (stale EventStopMovement _component) 0.1)
      (else
        (Variables|Default|SetDebug true)
        (Development|PrintString "Bloqueando")))))