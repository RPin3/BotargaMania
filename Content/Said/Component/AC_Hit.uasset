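; AC_Hit is a combo attack component that plays weak punch animations on sword input.
; Input plays the indexed sequence as an animation override on an AnimInstance supplied through the AnimationComponent event.
; Completion starts a timer and sets IsAttack, cancellation clears it, and both call AnimationSelect to increment the index.
; StopCombo resets the index, which has no wraparound, and the per-punch functions are empty stubs.
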(event Input|EnhancedActionEvents|EnhancedInputActionIA_Sword
  (params (ActionValue :type Boolean) (ElapsedSeconds :type Float%20%28double-precision%29) (TriggeredSeconds :type Float%20%28double-precision%29) (InputAction :type Input%20Action%20Object%20Reference :default "/Game/Charater2D/Input/Action/IA_Sword.IA_Sword"))
  (:Started
    (|PlayAnimationOverridewithCallbacks (Variables|/Script/PaperZD.PaperZDAnimationComponent|GetAnimInstance (Variables|Default|GetAnimation)) (Utilities|Array|Get(acopy) (Variables|Default|GetWeakPounchs) (Variables|Default|GetIndex)) "DefaultSlot" 1.0 0.0
      (:OnCompleted
        (Utilities|Time|SetTimerbyEvent (EventDispatchers|CreateEvent :!event StopCombo) 2.0)
        (Variables|Default|SetIsAttack true))
      (:OnCancelled
        (Variables|Default|SetIsAttack false)))
    (CallFunction|AnimationSelect)))

(event EventAnimationComponent
  (params (Animation :type Paper%20ZD%20Animation%20Component%20Object%20Reference))
  (Variables|Default|SetAnimation Animation))

(fn AnimationSelect
  (bind _output_get (Variables|Default|SetIndex (+ (Variables|Default|GetIndex) 1)))
  (switch int _output_get
    (:0
      (CallFunction|WeakPounch0))
    (:1
      (CallFunction|WeakPounch1))
    (:2
      (CallFunction|WeakPounch2))))

(fn StopCombo
  (Variables|Default|SetIndex 0))

(fn WeakPounch0)

(fn WeakPounch1)

(fn WeakPounch2)