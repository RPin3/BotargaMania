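; Actor component that detects directional key combos mapped to ability types.
; Movement records full left or right inputs in a buffer and sets a short timer, presumably bound to ResetCombo, which clears it.
; ComprobateCombo compares the buffer key by key against each ability's Combo1, returning the first full match's type or a default.
; Movement runs this check on each recorded input but leaves the result unused.
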(event Custom|ResetCombo
  (Utilities|Array|Clear (Variables|Default|Gettest)))

(event EventMovement
  (params (Input :type Float%20%28double-precision%29))
  (bind _test (Variables|Default|Gettest))
  (if (== Input -1.0)
    (Utilities|Array|Add _test (Variables|Default|GetLeft))
    (Utilities|Time|SetTimerbyEvent (EventDispatchers|CreateEvent :!event Custom|ResetCombo) 0.5 :!label _label)
    (CallFunction|ComprobateCombo (Variables|Default|Gettest))
    (elif (== Input 1.0)
      (Utilities|Array|Add _test (Variables|Default|GetRight))
      (goto _label))))

(fn ComprobateCombo
  (params (Input :type Array%20of%20Input%20Action%20Key%20Mapping%20Structures))
  (bind _array_element (Utilities|Array|ForEachLoopwithBreak (Variables|Default|GetListofAbilityes))
    (:LoopBody
      (bind (_array_element_2 _array_index) (Utilities|Array|ForEachLoopwithBreak Input :!label _label)
        (:LoopBody
          (if (== (Utilities|Struct|BreakInputActionKeyMapping _array_element_2) (Utilities|Struct|BreakInputActionKeyMapping (Utilities|Array|Get(acopy) (.Combo1 (Utilities|Struct|BreakAbilirties _array_element)) _array_index)))
            (Variables|Default|SetIndex (+ (Variables|Default|GetIndex) 1))
            (else
              (goto _label Break))))
        (:Completed
          (if (== (Variables|Default|GetIndex) (Utilities|Array|Length (.Combo1 (Utilities|Struct|BreakAbilirties _array_element))))
            (Variables|Default|SetIndex 0)
            (return (.TypeOfAbilitye (Utilities|Struct|BreakAbilirties _array_element)))
            (else
              (Variables|Default|SetIndex 0)
              (if (== _array_index (Utilities|Array|Length Input))
                _))))))
    (:Completed
      (Variables|Default|SetIndex 0)
      (return "NewEnumerator2"))))