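; BP_CharTest is a test character for trying out player and enemy health in the HUD.
; BeginPlay creates WB_UItest, adds it to the viewport and stores the reference.
; Keys 2 and 1 subtract a fixed amount from PlayerHealth and EnemyHealth respectively.
; The nodes that would write health into the widget's progress bars are disconnected, and Tick only calls its parent, so this graph never updates the bars.
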(event EventBeginPlay
  ;[0 0.7854 0.2265 0.5] Create HUD Widget and access to health properties to set percent into progress bars
  (|CallParentFunction)
  (bind _returnvalue (UserInterface|CreateWidget "/Game/Diego/HUD/WB_UItest.WB_UItest_C"))
  (UserInterface|Viewport|AddtoViewport _returnvalue 0)
  (Variables|Default|SetUIWidget _returnvalue))

(event Collision|EventActorBeginOverlap
  (params (OtherActor :type Actor%20Object%20Reference))
  (|CallParentFunction OtherActor) ; This node is disabled and will not be called.\nDrag off pins to build functionality.
)

(event EventTick
  (params (DeltaSeconds :type Float%20%28single-precision%29))
  ;[0.15 0.15 0.15 0.5] lo mismo que arriba xd
  (|CallParentFunction DeltaSeconds))

(event Input|KeyboardEvents|1
  (params (Key :type Key%20Structure))
  ;[0.6938 0 0.4399 0.5] Update health from enemy and player and set the values into each progress bar
  (:Pressed
    (bind _output_get (Variables|Default|SetEnemyHealth (- (Variables|Default|GetEnemyHealth) 1e+01)))))

(event Input|KeyboardEvents|2
  (params (Key :type Key%20Structure))
  ;[0.6938 0 0.4399 0.5] Update health from enemy and player and set the values into each progress bar
  (:Pressed
    (bind _output_get (Variables|Default|SetPlayerHealth (- (Variables|Default|GetPlayerHealth) 1e+01)))))

(fn ConstructionScript
  (|CallParentFunction))