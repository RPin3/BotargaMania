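; BP_AttackTest is a test player character with Enhanced Input jump, planar movement and an animated sword attack.
; The sword plays a PaperZD animation override and sets IsAttack, which blocks movement until it completes or is cancelled.
; A gate records horizontal input, passed to ACAbility when movement ends.
; CheckHit applies damage per Hitbox overlap and reports it to ACHealth; mapping-context setup, including a two-player attempt, is disconnected.
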(event Custom|StopMove
  (Variables|Default|SetMovement 0.0))

(event Custom|EneableInputPlayer
  (Input|EnableInput 0))

(event Input|EnhancedActionEvents|EnhancedInputActionIA_Move
  (params (ActionValue :type Vector%202D%20Structure) (ElapsedSeconds :type Float%20%28double-precision%29) (TriggeredSeconds :type Float%20%28double-precision%29) (InputAction :type Input%20Action%20Object%20Reference :default "/Game/Charater2D/Input/Action/IA_Move.IA_Move"))
  (bind (_x _y) (Math|Vector2D|BreakVector2D ActionValue))
  (:Triggered
    (if (CallFunction|CanAct)
      (Variables|Default|SetStop? false)
      (Pawn|Input|AddMovementInput "1.000000,0.000000,0.000000" _x false)
      (Pawn|Input|AddMovementInput "0.000000,1.000000,0.000000" _y false)
      (Utilities|FlowControl|Gate true :!label _label
        (:Exit
          (Variables|Default|SetMovement _x)))))
  (:Started
    (goto _label Open))
  (:Completed
    (Utilities|FlowControl|Sequence
      (:then_0
        (goto _label Close))
      (:then_1
        (Default|Movement (Variables|Default|GetAC_Ability) (Variables|Default|GetMovement))
        (Utilities|Time|SetTimerbyEvent (EventDispatchers|CreateEvent :!event Custom|StopMove) 0.1)))))

(event Input|EnhancedActionEvents|EnhancedInputActionIA_Sword
  (params (ActionValue :type Boolean) (ElapsedSeconds :type Float%20%28double-precision%29) (TriggeredSeconds :type Float%20%28double-precision%29) (InputAction :type Input%20Action%20Object%20Reference :default "/Game/Charater2D/Input/Action/IA_Sword.IA_Sword"))
  (:Started
    (|PlayAnimationOverridewithCallbacks (Variables|/Script/PaperZD.PaperZDAnimationComponent|GetAnimInstance (Variables|Default|GetAnimationComponent)) "/Game/Charater2D/Blueprints/KidPink/AnimSequences/Sowrd.Sowrd" "DefaultSlot" 1.0 0.0
      (:then
        (Variables|Default|SetIsAttack? true))
      (:OnCompleted
        (Variables|Default|SetIsAttack? false :!label _label))
      (:OnCancelled
        (goto _label)))))

(event Input|EnhancedActionEvents|EnhancedInputActionIA_Jump
  (params (ActionValue :type Boolean) (ElapsedSeconds :type Float%20%28double-precision%29) (TriggeredSeconds :type Float%20%28double-precision%29) (InputAction :type Input%20Action%20Object%20Reference :default "/Game/Charater2D/Input/Action/IA_Jump.IA_Jump"))
  (:Started
    (Character|Jump))
  (:Completed
    (Character|StopJumping)))

(event EventBeginPlay)

(event EventDisableInputPlayer
  (params (Time :type Float%20%28double-precision%29))
  (Input|DisableInput 0)
  (Utilities|Time|SetTimerbyEvent (EventDispatchers|CreateEvent :!event Custom|EneableInputPlayer) Time))

(fn ConstructionScript)

(fn CanAct
  (return (not (Variables|Default|GetIsAttack?))))

(fn CheckHit
  (for _array_element (Collision|GetOverlappingActors (Variables|Default|GetHitbox) "/Script/Engine.Actor" :!class /Script/Engine.PrimitiveComponent)
    (bind _returnvalue (Game|Damage|ApplyDamage 0 (Variables|Default|GetDamage) 0 0 "/Script/Engine.DamageType"))
    (Class|BPIHealth|DamageHealth(Message) (Variables|Default|GetAC_Health) _returnvalue)))