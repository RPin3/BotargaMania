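; GM_KidPink is a game mode Blueprint containing a draft local two-player setup, currently disconnected, so BeginPlay does nothing.
; The unwired logic loops over every PlayerStart, creates a local player and spawns a BP_AttackTest pawn there for possession.
; It adds IMC_Player1 for the first player and IMC_Player2 for any later ones, giving each separate Enhanced Input mappings.
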(event EventBeginPlay)

(fn ConstructionScript)