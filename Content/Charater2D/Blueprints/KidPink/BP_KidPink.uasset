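; Player character Blueprint for KidPink, a 2D-animated kid driven by Enhanced Input for jumping and movement.
; Movement is blocked while attacking or dead, and a gate forwards its direction to health and ability components.
; CheckHit sends hitbox damage and VFX, while capsule collisions spawn and trigger a short-lived MF_Base actor.
; A debug key self-damages, playing a hit override animation and jumping to another animation node on death.
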(event OnComponentHit(CapsuleComponent)
  (params (HitComponent :type Primitive%20Component%20Object%20Reference) (OtherActor :type Actor%20Object%20Reference) (OtherComp :type Primitive%20Component%20Object%20Reference) (NormalImpulse :type Vector :default "0, 0, 0") (Hit :type Hit%20Result%20Structure%20%28by%20ref%29))
  (bind _impactpoint (Collision|BreakHitResult Hit))
  (bind _returnvalue (Math|Conversions|ToTransform(Vector) _impactpoint))
  (bind _returnvalue_2 (Game|SpawnActorfromClass "/Game/Jhony/Chaos/GC/MF_Base.MF_Base_C" (Math|Transform|MakeTransform (.location _returnvalue) (.rotation _returnvalue) "0.300000,0.350000,0.350000") "Undefined" "MultiplyWithRoot" 0 0))
  (bind _output_get (Variables|Default|SetMF _returnvalue_2))
  (Variables|/Engine/EditorResources/FieldNodes/FS_MasterField.FS_MasterField_C|SetActivationType _output_get "NewEnumerator4")
  (Actor|SetLifeSpan (Variables|Default|GetMF) 0.2)
  (Default|CETrigger (Variables|Default|GetMF)))

(event Custom|StopMove
  (bind _output_get (Variables|Default|SetMovement 0.0))
  (Default|StopMovement (Variables|Default|GetAC_Health) _output_get))

(event Custom|EneableInputPlayer
  (Input|EnableInput 0))

(event Custom|DamageHitAnim)

(event Input|EnhancedActionEvents|EnhancedInputActionIA_Jump
  (params (ActionValue :type Boolean) (ElapsedSeconds :type Float%20%28double-precision%29) (TriggeredSeconds :type Float%20%28double-precision%29) (InputAction :type Input%20Action%20Object%20Reference :default "/Game/Charater2D/Input/Action/IA_Jump.IA_Jump"))
  (:Started
    (Character|Jump))
  (:Completed
    (Character|StopJumping)))

(event Input|EnhancedActionEvents|EnhancedInputActionIA_Move
  (params (ActionValue :type Vector%202D%20Structure) (ElapsedSeconds :type Float%20%28double-precision%29) (TriggeredSeconds :type Float%20%28double-precision%29) (InputAction :type Input%20Action%20Object%20Reference :default "/Game/Charater2D/Input/Action/IA_Move.IA_Move"))
  (bind (_x _y) (Math|Vector2D|BreakVector2D ActionValue))
  ;[0.5938 0.5938 0.5938 0.5] Movement
  (:Triggered
    (if (CallFunction|Canattack)
      (Variables|Default|SetStop? false)
      (Pawn|Input|AddMovementInput "1.000000,0.000000,0.000000" _x false)
      (Pawn|Input|AddMovementInput "0.000000,1.000000,0.000000" _y false)
      (Utilities|FlowControl|Gate true :!label _label
        (:Exit
          (bind _output_get (Variables|Default|SetMovement _x))
          (Default|DirectionMovement (Variables|Default|GetAC_Health) _output_get)))))
  (:Started
    (goto _label Open))
  (:Completed
    (Utilities|FlowControl|Sequence
      (:then_0
        (goto _label Close))
      (:then_1
        (Default|Movement (Variables|Default|GetAC_Ability) (Variables|Default|GetMovement))
        (Utilities|Time|SetTimerbyEvent (EventDispatchers|CreateEvent :!event Custom|StopMove) 0.1)))))

(event EventBeginPlay
  (Utilities|FlowControl|Sequence
    (:then_0
      (bind _asplayer_controller (Utilities|Casting|CastToPlayerController (Pawn|GetController)))
      (Input|AddMappingContext (PlayerController|LocalPlayerSubsystems|GetEnhancedInputLocalPlayerSubsystem _asplayer_controller) "/Game/Charater2D/Input/IMC_Player1.IMC_Player1" 0 "(bIgnoreAllPressedKeysUntilRelease=True,bForceImmediately=False,bNotifyUserSettings=False)"))
    (:then_1
      (bind _component (CallFunction|FindComponentbyInterface self "/Game/Said/Interface/BPI_Components.BPI_Components_C"))
      (Class|BPIComponents|AnimationComponent(Message) _component (Variables|Default|GetAnimationComponent)))))

(event EventDisableInputPlayer
  (params (Time :type Float%20%28double-precision%29))
  (Input|DisableInput 0)
  (Utilities|Time|SetTimerbyEvent (EventDispatchers|CreateEvent :!event Custom|EneableInputPlayer) Time))

(event Input|KeyboardEvents|DebugKeyM
  (params (Key :type Key%20Structure :default "None") (ActionValue :type Input%20Action%20Value%20Structure))
  (:Pressed
    (Default|DamageHealth (Variables|Default|GetAC_Health) 1e+01)
    (|PlayAnimationOverridewithCallbacks (Variables|/Script/PaperZD.PaperZDAnimationComponent|GetAnimInstance (Variables|Default|GetAnimationComponent)) (Variables|Default|GetHit%20anim%20sequence) (Variables|Default|GetHit%20Slot%20Name) 1.0 0.0
      (:OnCompleted
        _)
      (:OnCancelled
        _))
    (if (Variables|/Game/Said/Component/AC_Health.AC_Health_C|GetIsDead (Variables|Default|GetAC_Health))
      (Class|PaperZDAnimInstance|JumptoNode (Variables|/Script/PaperZD.PaperZDAnimationComponent|GetAnimInstance (Variables|Default|GetAnimationComponent)) (Variables|Default|GetJump%20Name) "None"))))

(fn ConstructionScript)

(fn Canattack
  (return (and (not (Variables|Default|GetIsAttack)) (not (Variables|/Game/Said/Component/AC_Health.AC_Health_C|GetIsDead (Variables|Default|GetAC_Health))))))

(fn CheckHit
  (params (Damage :type Float%20%28double-precision%29))
  (for _array_element (Collision|GetOverlappingActors (Variables|Default|GetHitbox) "/Script/Engine.Actor" :!class /Script/Engine.PrimitiveComponent)
    (Class|BPIHealth|DamageHealth(Message) (Variables|Default|GetAC_Health) Damage)
    (Default|CustomVFX (Variables|Default|GetAC_HitVFX) (Math|Conversions|ToTransform(Vector) (Transformation|GetWorldLocation (Variables|Default|GetHitBox))) "/Game/Said/VFX/Prueba.Prueba_C")))